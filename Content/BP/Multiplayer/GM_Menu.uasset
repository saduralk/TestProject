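; GM_Menu is the menu game mode that tracks connected players for a multiplayer lobby and shares their profiles.
; New-player handling adds player controller 0, cast to BP_MenuController, to ConnectedPlayers.
; UpdateLobby triggers CauseLobbyUpdate, which rebuilds PlayerProfiles from valid controllers and pushes the list to each through UpdatePlayerNames.
; Getters expose the connected players and a connection type, while ReturnPlayerProfile is an empty stub.
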(event Custom|Cause%20Lobby%20Update
  (params (Update%20Names? :type Boolean))
  (if Update%20Names?
    (Utilities|Array|Clear (Variables|Default|GetPlayer%20Profiles))
    (for _array_element (Variables|Default|GetConnectedPlayers)
      (Utilities|IsValid _array_element
        (:Is%20Valid
          (Utilities|Array|Add (Variables|Default|GetPlayer%20Profiles) (Variables|/Game/BP/Multiplayer/BP_MenuController.BP_MenuController_C|GetPlayer%20Profile%20Info _array_element)))))
    (for _array_element_2 (Variables|Default|GetConnectedPlayers)
      (if Update%20Names?
        (Utilities|IsValid _array_element_2
          (:Is%20Valid
            (Default|UpdatePlayerNames _array_element_2 (Variables|Default|GetPlayer%20Profiles))))))))

(event EventBeginPlay)

(event EventTick
  (params (DeltaSeconds :type Float%20%28single-precision%29)))

(event EventUpdateLobby
  (CallFunction|CauseLobbyUpdate true))

(event EventHandleStartingNewPlayer
  (params (NewPlayer :type Player%20Controller%20Object%20Reference))
  (bind _returnvalue (Game|GetCurrentLevelName true))
  (switch string _returnvalue
    (:LVL_Lobby
      (Utilities|Array|Add (Variables|Default|GetConnectedPlayers) (.AsBP%20Menu%20Controller (Utilities|Casting|CastToBP_MenuController (Game|GetPlayerController 0)))))))

(fn ConstructionScript)

(fn GetConnectionType
  (return "Value1"))

(fn RetrieveConnectedPlayers
  (return (Variables|Default|GetConnectedPlayers)))

(fn ReturnPlayerProfile
  (return ""))