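; Multiplayer menu controller that syncs the player's saved profile with the lobby and manages the lobby widget.
; RunSetup loads the profile from an SG_Multiplayer save, creating one if missing, then passes it to ServerSideUpdateLobby, which stores it and notifies the GameMode.
; Other events show the lobby widget with a mouse cursor and refresh its player names.
; Connection type and player/profile getters are placeholder stubs.
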(event Custom|Initial%20Setup
  (CallFunction|LoadSavedProfile))

(event Custom|Server%20Side%20Update%20Lobby
  (params (Player%20Profile :type Player%20Profile%20Structure))
  (Variables|Default|SetPlayer%20Profile%20Info Player%20Profile)
  (Class|BPIMultiplayer|UpdateLobby(Message) (Game|GetGameMode)))

(event Custom|Update%20Player%20Names
  (params (Player%20Profile :type Array%20of%20Player%20Profile%20Structures))
  (bind _lobby_menu (Variables|Default|GetLobby%20Menu))
  (Default|ClearPlayerNames _lobby_menu)
  (Default|UpdatePlayerNames _lobby_menu Player%20Profile))

(event EventBeginPlay)

(event EventTick
  (params (DeltaSeconds :type Float%20%28single-precision%29)))

(event EventRunSetup
  (CallFunction|InitialSetup)
  (CallFunction|ServerSideUpdateLobby (Variables|Default|GetPlayer%20Profile%20Info)))

(event EventShowtheLobby
  (CallFunction|ShowLobbyMenu))

(fn ConstructionScript)

(fn LoadSavedProfile
  (bind _returnvalue (SaveGame|DoesSaveGameExist (LocalVariables|GetPlayer%20Profile%20Slot)))
  (if _returnvalue
    _
    (else
      (bind _returnvalue_2 (SaveGame|CreateSaveGameObject "/Game/BP/Multiplayer/SG_Multiplayer.SG_Multiplayer_C"))
      (SaveGame|SaveGametoSlot _returnvalue_2 (LocalVariables|GetPlayer%20Profile%20Slot))))
  (bind _returnvalue_3 (SaveGame|LoadGamefromSlot (LocalVariables|GetPlayer%20Profile%20Slot)))
  (bind _player_profile (Class|BPIMultiplayer|ReturnPlayerProfile(Message) _returnvalue_3))
  (Variables|Default|SetPlayer%20Profile%20Info _player_profile)
  (return))

(fn ShowLobbyMenu
  (Utilities|IsValid (Variables|Default|GetLobby%20Menu)
    (:Is%20Valid
      _)
    (:Is%20Not%20Valid
      (bind _returnvalue (UserInterface|CreateWidget "/Game/BP/Multiplayer/LobbyMenu_WBP.LobbyMenu_WBP_C"))
      (bind _output_get (Variables|Default|SetLobby%20Menu _returnvalue))))
  (UserInterface|Viewport|AddtoViewport _output_get 0)
  (Variables|/Script/Engine.PlayerController|SetbShowMouseCursor (Game|GetPlayerController 0) true))

(fn GetConnectionType
  (return "Value1"))

(fn RetrieveConnectedPlayers
  (return 0))

(fn ReturnPlayerProfile
  (return ""))